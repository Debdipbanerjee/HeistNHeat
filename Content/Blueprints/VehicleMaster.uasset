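; VehicleMaster is a vehicle Blueprint that routes two sets of driving inputs to a RaceCar and a PoliceCar2.
; BeginPlay starts its own engine and caches both cars by class lookup.
; Separate axis and handbrake inputs drive each car, with throttle sign setting shifter position; shifter events are duplicated for both.
; Launch spawns a Missle_BP at the police car's launch point, then turns its launcher toward the race car.
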(event EventBeginPlay
  (|CallParentFunction)
  (CallFunction|StartEngine)
  (CallFunction|SetShifterPosition "NewEnumerator3")
  (Utilities|FlowControl|Sequence
    (:then_0
      (bind _returnvalue (Actor|GetActorOfClass "/Game/Blueprints/RaceCar.RaceCar_C")))
    (:then_1
      (bind _returnvalue_2 (Actor|GetActorOfClass "/Game/Blueprints/PoliceCar2.PoliceCar2_C")))))

(event Input|ActionEvents|InputActionShifterUp
  (params (Key :type Key%20Structure :default "None"))
  ;[1 1 1] Shifter
  (:Pressed
    (Default|MoveShifterPosition (stale EventBeginPlay _returnvalue_2) false)))

(event Input|ActionEvents|InputActionHandBrake
  (params (Key :type Key%20Structure :default "None"))
  (:Pressed
    (Default|SetHandbrakeInput (stale EventBeginPlay _returnvalue) true))
  (:Released
    (Default|SetHandbrakeInput (stale EventBeginPlay _returnvalue) false)))

(event Input|ActionEvents|InputActionLaunch
  (params (Key :type Key%20Structure :default "None"))
  (:Pressed
    (Actor|GetActorOfClass "/Game/Blueprints/RaceCar.RaceCar_C")
    (Game|SpawnActorfromClass "/Game/Blueprints/Missle/Missle_BP.Missle_BP_C" (Math|Transform|MakeTransform (Transformation|GetWorldLocation (Variables|/Game/Blueprints/PoliceCar2.PoliceCar2_C|GetLaunchPoint (stale EventBeginPlay _returnvalue_2))) "0, 0, 0" "1,1,1") "Undefined" 0 0)
    (bind _returnvalue (Actor|GetActorOfClass "/Game/Blueprints/PoliceCar2.PoliceCar2_C"))
    (Transformation|SetWorldRotation (Variables|/Game/Blueprints/PoliceCar2.PoliceCar2_C|GetLauncher _returnvalue) (Math|Conversions|RotationFromXVector (Math|Rotator|GetRotationXVector (Math|Rotator|FindLookatRotation (Transformation|GetWorldLocation (Variables|/Game/Blueprints/PoliceCar2.PoliceCar2_C|GetLauncher _returnvalue)) (Transformation|GetActorLocation (stale EventBeginPlay _returnvalue))))) false false)))

(event Input|ActionEvents|InputActionShifterDown
  (params (Key :type Key%20Structure :default "None"))
  ;[1 1 1] Shifter
  (:Pressed
    (Default|MoveShifterPosition (stale EventBeginPlay _returnvalue_2) false)))

(event Input|ActionEvents|InputActionHandBrake2
  (params (Key :type Key%20Structure :default "None"))
  (:Pressed
    (Default|SetHandbrakeInput (stale EventBeginPlay _returnvalue_2) true))
  (:Released
    (Default|SetHandbrakeInput (stale EventBeginPlay _returnvalue_2) false)))

(event Input|ActionEvents|InputActionShifterUp
  (params (Key :type Key%20Structure :default "None"))
  ;[1 1 1] Shifter
  (:Pressed
    (Default|MoveShifterPosition (stale EventBeginPlay _returnvalue) false)))

(event Input|ActionEvents|InputActionShifterDown
  (params (Key :type Key%20Structure :default "None"))
  ;[1 1 1] Shifter
  (:Pressed
    (Default|MoveShifterPosition (stale EventBeginPlay _returnvalue) false)))

(event Input|AxisEvents|InputAxisMoveForward
  (params (AxisValue :type Float%20%28single-precision%29))
  ;[1 1 1] Throttle/Steering
  (if (>= AxisValue 0.0)
    (Default|SetShifterPosition (stale EventBeginPlay _returnvalue_2) "NewEnumerator3")
    (else
      (Default|SetShifterPosition (stale EventBeginPlay _returnvalue_2) "NewEnumerator1")))
  (Default|SetThrottleInput (stale EventBeginPlay _returnvalue_2) AxisValue))

(event Input|AxisEvents|InputAxisMoveRight
  (params (AxisValue :type Float%20%28single-precision%29))
  ;[1 1 1] Throttle/Steering
  (Default|SetSteeringInput (stale EventBeginPlay _returnvalue_2) AxisValue))

(event Input|AxisEvents|InputAxisVehicleForward
  (params (AxisValue :type Float%20%28single-precision%29))
  ;[1 1 1] Throttle/Steering
  (if (>= AxisValue 0.0)
    (Default|SetShifterPosition (stale EventBeginPlay _returnvalue) "NewEnumerator3")
    (else
      (Default|SetShifterPosition (stale EventBeginPlay _returnvalue) "NewEnumerator1")))
  (Default|SetThrottleInput (stale EventBeginPlay _returnvalue) AxisValue))

(event Input|AxisEvents|InputAxisVehicleSteering
  (params (AxisValue :type Float%20%28single-precision%29))
  ;[1 1 1] Throttle/Steering
  (Default|SetSteeringInput (stale EventBeginPlay _returnvalue) AxisValue))

(fn ConstructionScript
  (|CallParentFunction))