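; PoliceCar is a drivable car Blueprint that turns player input into engine, shifter, throttle and steering calls.
; BeginPlay starts the engine and sets an initial shifter position.
; The MoveForward axis picks the shifter position by sign, feeds the throttle and prints a debug string, while MoveRight feeds steering.
; ShifterUp and ShifterDown both call MoveShifterPosition with the same false argument.
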(event EventBeginPlay
  (|CallParentFunction)
  (CallFunction|StartEngine)
  (CallFunction|SetShifterPosition "NewEnumerator3"))

(event Input|ActionEvents|InputActionShifterUp
  (params (Key :type Key%20Structure :default "None"))
  (:Pressed
    (CallFunction|MoveShifterPosition false)))

(event Input|ActionEvents|InputActionShifterDown
  (params (Key :type Key%20Structure :default "None"))
  (:Pressed
    (CallFunction|MoveShifterPosition false)))

(event Input|AxisEvents|InputAxisMoveForward
  (params (AxisValue :type Float%20%28single-precision%29))
  (if (>= AxisValue 0.0)
    (CallFunction|SetShifterPosition "NewEnumerator3")
    (else
      (CallFunction|SetShifterPosition "NewEnumerator1")))
  (CallFunction|SetThrottleInput AxisValue)
  (Development|PrintString "Hello"))

(event Input|AxisEvents|InputAxisMoveRight
  (params (AxisValue :type Float%20%28single-precision%29))
  (CallFunction|SetSteeringInput AxisValue))

(fn ConstructionScript
  (|CallParentFunction))