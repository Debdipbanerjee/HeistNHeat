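; Camera actor that frames a race car and a police car together.
; On BeginPlay it finds one RaceCar and one PoliceCar2 by class.
; Each tick it places its camera at their midpoint, offset along world X and Z by their separation times tunable multipliers, pulling back as the cars spread apart.
; A default distance sets the minimum offset, and only location is updated, not rotation.
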(event EventTick
  (params (DeltaSeconds :type Float%20%28single-precision%29))
  (bind _defaultdis (Variables|Default|GetDefaultDis))
  (if (> (Math|Vector|Distance(Vector) (Transformation|GetActorLocation (stale EventBeginPlay _returnvalue)) (Transformation|GetActorLocation (stale EventBeginPlay _returnvalue_2))) (Variables|Default|GetDefaultDis))
    (Transformation|SetWorldLocation (Variables|CameraActor|GetCameraComponent) (+ (+ (/ (+ (Transformation|GetActorLocation (stale EventBeginPlay _returnvalue)) (Transformation|GetActorLocation (stale EventBeginPlay _returnvalue_2))) 2.0) (* "1.000000, 0, 0" (* (Math|Vector|Distance(Vector) (Transformation|GetActorLocation (stale EventBeginPlay _returnvalue)) (Transformation|GetActorLocation (stale EventBeginPlay _returnvalue_2))) (Variables|Default|GetXval)))) (* "0.000000, 0,1.000000" (* (Math|Vector|Distance(Vector) (Transformation|GetActorLocation (stale EventBeginPlay _returnvalue)) (Transformation|GetActorLocation (stale EventBeginPlay _returnvalue_2))) (Variables|Default|GetZval)))) false false)
    (else
      (Transformation|SetWorldLocation (Variables|CameraActor|GetCameraComponent) (+ (/ (+ (Transformation|GetActorLocation (stale EventBeginPlay _returnvalue)) (Transformation|GetActorLocation (stale EventBeginPlay _returnvalue_2))) 2.0) (Math|Vector|MakeVector (* (Variables|Default|GetXval) _defaultdis) 0.0 (* _defaultdis (Variables|Default|GetZval)))) false false))))

(event EventBeginPlay
  (Utilities|FlowControl|Sequence
    (:then_0
      (bind _returnvalue (Actor|GetActorOfClass "/Game/Blueprints/RaceCar.RaceCar_C")))
    (:then_1
      (bind _returnvalue_2 (Actor|GetActorOfClass "/Game/Blueprints/PoliceCar2.PoliceCar2_C")))))

(fn ConstructionScript)