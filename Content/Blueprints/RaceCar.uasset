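; Race car Blueprint that adds a timed speed boost and caps the vehicle's velocity.
; Full Boost axis input sets a boosting flag, shows exhaust and wind effects, applies pitch-up rotation to the mesh, then clears flag and effects after chained delays.
; Tick overwrites physics velocity directly, scaling it up per frame toward the boost cap while boosting and otherwise clamping it to normal max speed.
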(event EventTick
  (params (DeltaSeconds :type Float%20%28single-precision%29))
  (bind _returnvalue (Transformation|GetVelocity))
  (bind _returnvalue_2 (Transformation|GetVelocity))
  (bind _maxspeed (Variables|Default|GetMaxSpeed))
  (bind _maxboostspeed (Variables|Default|GetMaxBoostSpeed))
  (Utilities|FlowControl|Sequence
    (:then_0
      (if (Variables|Default|GetIsBoosting)
        (if (> (Math|Vector|VectorLength _returnvalue_2) _maxboostspeed)
          (Physics|SetPhysicsLinearVelocity (Variables|Default|GetVehicleMesh) (* (Math|Vector|Normalize _returnvalue_2) _maxboostspeed) false "None")
          (else
            (Physics|SetPhysicsLinearVelocity (Variables|Default|GetVehicleMesh) (* (Transformation|GetVelocity) 1.01) false "None")))
        (elif (> (Math|Vector|VectorLength _returnvalue) _maxspeed)
          (Physics|SetPhysicsLinearVelocity (Variables|Default|GetVehicleMesh) (* (Math|Vector|Normalize _returnvalue) _maxspeed) false "None"))))))

(event Input|AxisEvents|InputAxisBoost
  (params (AxisValue :type Float%20%28single-precision%29))
  (bind _vehiclemesh (Variables|Default|GetVehicleMesh))
  (bind _vehiclemesh_2 (Variables|Default|GetVehicleMesh))
  (bind _returnvalue (Transformation|GetWorldRotation _vehiclemesh_2))
  (bind _returnvalue_2 (Transformation|GetWorldRotation _vehiclemesh))
  (bind _returnvalue_3 (Math|Rotator|GetRotationXVector (Math|Rotator|MakeRotator (.roll _returnvalue) (.pitch _returnvalue) (.yaw _returnvalue))))
  (bind _returnvalue_4 (Math|Rotator|GetRotationXVector (Math|Rotator|MakeRotator (.roll _returnvalue_2) (.pitch _returnvalue_2) (.yaw _returnvalue_2))))
  (if (== AxisValue 1.0)
    (Variables|Default|SetIsBoosting true)
    (Transformation|AddRelativeRotation (Variables|Default|GetVehicleMesh) (Math|Rotator|MakeRotator (.x _returnvalue_3) 2.0 (.z _returnvalue_3)) false false)
    (Rendering|SetVisibility (Variables|Default|GetExhaust) true false)
    (Utilities|FlowControl|Delay 1.0)
    (Transformation|AddRelativeRotation (Variables|Default|GetVehicleMesh) (Math|Rotator|MakeRotator (.x _returnvalue_4) 0.0 (.z _returnvalue_4)) false false)
    (Utilities|FlowControl|Delay 2.0)
    (Rendering|SetVisibility (Variables|Default|GetExhaust) false false)
    (Variables|Default|SetIsBoosting false)))

(fn ConstructionScript
  (|CallParentFunction))